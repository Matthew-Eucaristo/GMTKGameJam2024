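; Player balloon that flies on gas held in the game mode, winning if it pops on the target BP_BapakBocah and losing on other hits or empty gas.
; Mic loudness or Space presses generate gas, which Tick burns for size-scaled forward velocity and uses to scale the balloon.
; Move input spends gas to steer, while timer-randomized sine wind drifts heading.
; Construction builds an instanced-mesh and spline-mesh chain, but its follow update never runs.
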(event `Change the Randomness of the Wind`
  (set `self.Wind Direction Randomizer` (`KismetMathLibrary.RandomIntegerInRange` 0 6))
  (set `self.Balloon Wind Direction Multiplier` (`KismetMathLibrary.RandomFloatInRange` -2.0 2.0)))

(event `self.ReceiveBeginPlay`
  (`|ExecutionSequence`
    (:`then_0`
      ;[1 1 1] Setting up necessary references
      (bind _asbp_game_mode_main (cast `/Game/Blueprints/BP_GameModeMain` (`GameplayStatics.GetGameMode`)))
      (set `self.As BP Game Mode Main` _asbp_game_mode_main)
      (bind _asgi_game_instance_main (cast `/Game/Blueprints/GI_GameInstanceMain` (`GameplayStatics.GetGameInstance`)))
      (set `self.As GI Game Instance Main` _asgi_game_instance_main))
    (:`then_1`
      (`KismetSystemLibrary.K2_SetTimerDelegate` (delegate `Change the Randomness of the Wind`) (`KismetMathLibrary.RandomFloatInRange` 2.0 4.0) true))))

(event `self.ReceiveTick`
  (params (DeltaSeconds :type "Float (single-precision)"))
  (bind _returnvalue (* (`self.Balloon Wind Direction Multiplier`) (`KismetMathLibrary.Sin` (`KismetSystemLibrary.GetGameTimeInSeconds`))))
  (`|ExecutionSequence`
    (:`then_0`
      ;[1 1 1] Call Gas basic mechanics
      (`self.Try to Generate GAs`)
      (`self.Consume Gas Energy to Move Forward`)
      (`self.Scale Player base on Gas`))
    (:`then_1`
      (`SceneComponent.K2_AddWorldRotation` (`self.Baloon Direction`) (select `int` (`self.Wind Direction Randomizer`) :`0` (`KismetMathLibrary.MakeRotator` _returnvalue) :`1` (`KismetMathLibrary.MakeRotator` 0.0 _returnvalue) :`2` (`KismetMathLibrary.MakeRotator` 0.0 0.0 _returnvalue) :`3` (`KismetMathLibrary.MakeRotator` _returnvalue _returnvalue) :`4` (`KismetMathLibrary.MakeRotator` 0.0 _returnvalue _returnvalue) :`5` (`KismetMathLibrary.MakeRotator` _returnvalue 0.0 _returnvalue) :`6` (`KismetMathLibrary.MakeRotator` _returnvalue _returnvalue _returnvalue)) false false))))

(event `LerpLocation`
  (bind (_returnvalue_location _returnvalue_rotation) (`KismetMathLibrary.BreakTransform` (`self.GetTransform`)))
  (bind _ism (`self.ISM`))
  (bind (_output_location _output_rotation _output_scale) (`KismetMathLibrary.BreakTransform` (`|GetArrayItem` (`self.Instance Transform`))))
  (`KismetArrayLibrary.Array_Clear` (`self.Instance Transform`))
  (for _index (range (`InstancedStaticMeshComponent.GetInstanceCount` (`self.ISM`)))
    (`KismetArrayLibrary.Array_Add` (`self.Instance Transform`) (`InstancedStaticMeshComponent.GetInstanceTransform` (`self.ISM`) _index true)))
  (`InstancedStaticMeshComponent.UpdateInstanceTransform` (`self.ISM`) 0 (`KismetMathLibrary.MakeTransform` _returnvalue_location _returnvalue_rotation _output_scale) true true false)
  (for (_array_element _array_index) (`self.Instance Transform`)
    (bind _returnvalue (+ _array_index 1))
    (`InstancedStaticMeshComponent.UpdateInstanceTransform` _ism _returnvalue (`KismetMathLibrary.TLerp` (`InstancedStaticMeshComponent.GetInstanceTransform` _ism _returnvalue true) _array_element 0.075) true true false)))

(event `Scale Player base on Gas`
  ;[1 1 1] Update Player Scaling by sizes
  (`self.SetActorScale3D` (`KismetMathLibrary.VLerp` (`self.GetActorScale3D`) (`KismetMathLibrary.VLerp` (0.5 0.5 0.5) (4.0 4.0 4.0) (`/Game/Blueprints/BP_GameModeMain.Gas Energy` (`self.As BP Game Mode Main`))) 0.2)))

(event `Consume Gas Energy to Move Forward`
  (bind _returnvalue_x (`KismetMathLibrary.BreakVector` (`self.GetActorScale3D`)))
  (bind _capsulecomponent (`self.CapsuleComponent`))
  ;[1 1 1] Handle Moving Forward
  (`KismetSystemLibrary.Delay` 0.1)
  (bind _succeed (`/Game/Blueprints/BP_GameModeMain.Consume Gas` (`self.As BP Game Mode Main`) 0.005))
  (if _succeed
    (bind _returnvalue (`PrimitiveComponent.GetPhysicsLinearVelocity` _capsulecomponent "None"))
    (`PrimitiveComponent.SetPhysicsLinearVelocity` _capsulecomponent (`KismetMathLibrary.VLerp` _returnvalue (* (`SceneComponent.GetForwardVector` (`self.Baloon Direction`)) (* (`self.Base Speed`) _returnvalue_x)) 0.5) false "None")
    (else
      (`/Game/Blueprints/GI_GameInstanceMain.Lose Game` (`self.As GI Game Instance Main`)))))

(event `Try to Generate Gas`
  (bind _as_bp_game_mode_main (`self.As BP Game Mode Main`))
  (bind _space_bar_pressed_in_certain_checks (`self.Space Bar Pressed in certain checks`))
  (bind _as_bp_game_mode_main_2 (`self.As BP Game Mode Main`))
  (bind _player_volume (`self.Player Volume`))
  (`KismetSystemLibrary.Delay` 0.15) ; how fast the checking and gas generation
  (if (`self.Player Use Mic`)
    ;[1 1 1] Handling Gas Generation using Mic
    (if (> _player_volume 0.95)
      (`/Game/Blueprints/BP_GameModeMain.Generate Gas` _as_bp_game_mode_main_2 (`self.Extreme Gas Generation`))
      (`KismetSystemLibrary.PrintString` "SLOW WE")
      (elif (> _player_volume 0.5)
        (`/Game/Blueprints/BP_GameModeMain.Generate Gas` _as_bp_game_mode_main_2 (`self.Normal Gas Generation`))
        (`KismetSystemLibrary.PrintString` "Gas Generated")))
    (else
      ;[1 1 1] Handling Gas Generation using Space Bar
      (if (> _space_bar_pressed_in_certain_checks 2)
        (`/Game/Blueprints/BP_GameModeMain.Generate Gas` _as_bp_game_mode_main (`self.Extreme Gas Generation`))
        (`KismetSystemLibrary.PrintString` "SLOW WE")
        (set `self.Space Bar Pressed in certain checks` 0 :!label _label) ; reset space bar count
        (elif (> _space_bar_pressed_in_certain_checks 0)
          (`/Game/Blueprints/BP_GameModeMain.Generate Gas` _as_bp_game_mode_main (`self.Normal Gas Generation`))
          (`KismetSystemLibrary.PrintString` "Gas Generated")
          (goto _label))))))

(event `Key|SpaceBar`
  (params (Key :type "Key Structure"))
  ;[1 1 1] Just to handle if player doesn't choose Mic
  (:`Pressed`
    (if (not (`self.Player Use Mic`))
      (`/Engine/EditorBlueprintResources/StandardMacros.IncrementInt` (`self.Space Bar Pressed in certain checks`)))))

(event `EnhancedInput|/Game/Blueprints/Inputs/InputActions/IA_Move`
  (params (ActionValue :type "Vector2D Structure") (ElapsedSeconds :type "Float (double-precision)") (TriggeredSeconds :type "Float (double-precision)") (InputAction :type "InputAction Object Reference" :default "/Game/Blueprints/Inputs/InputActions/IA_Move.IA_Move"))
  (bind _returnvalue_x (`KismetMathLibrary.BreakVector` (`self.GetActorScale3D`)))
  (bind _baloon_direction (`self.Baloon Direction`))
  (:`Triggered`
    (`KismetSystemLibrary.Delay` 0.03)
    (bind _succeed (`/Game/Blueprints/BP_GameModeMain.Consume Gas` (`self.As BP Game Mode Main`) 0.003))
    (if _succeed
      (`SceneComponent.K2_AddRelativeRotation` _baloon_direction (`KismetMathLibrary.MakeRotator` 0.0 (* ActionValue_Y 10.0) (* ActionValue_X 10.0)) false false)
      (`PrimitiveComponent.AddImpulse` (`self.CapsuleComponent`) (* (`SceneComponent.GetForwardVector` _baloon_direction) (* (`self.Turn Impulse Power`) _returnvalue_x)) "None" false)
      (else
        (`KismetSystemLibrary.PrintString` "ENTEK WE" true true (struct :`R` 0.836177 :`B` 1.0 :`A` 1.0))))))

(event `self.AudioCapture.OnAudioEnvelopeValue`
  (params (EnvelopeValue :type "Float (single-precision)"))
  ;[1 1 1] Handling Audio Capture
  (set `self.Player Volume` (`KismetMathLibrary.FClamp` (`KismetMathLibrary.NormalizeToRange` EnvelopeValue 0.0 0.1))))

(event `self.CapsuleComponent.OnComponentHit`
  (params (HitComponent :type "PrimitiveComponent Object Reference") (OtherActor :type "Actor Object Reference") (OtherComp :type "PrimitiveComponent Object Reference") (NormalImpulse :type "Vector Structure") (Hit :type "HitResult Structure (by ref)"))
  (bind _as_gi_game_instance_main (`self.As GI Game Instance Main`))
  (`/Engine/EditorBlueprintResources/StandardMacros.DoOnce` false
    (:`Completed`
      (`NiagaraFunctionLibrary.SpawnSystemAtLocation` "/Game/Niagara/NS_POP.NS_POP" (`self.K2_GetActorLocation`) (struct) (0.05 0.05 0.05))
      (`SceneComponent.SetVisibility` (`self.Sphere_Mesh`) false false)
      (bind _asbp_bapak_bocah (cast `/Game/Blueprints/Siswa/BP_BapakBocah` OtherActor)
        (:`then`
          (if (`/Game/Blueprints/Siswa/BP_BapakBocah.Is Target` _asbp_bapak_bocah)
            (`/Game/Blueprints/GI_GameInstanceMain.Win Game` _as_gi_game_instance_main)
            (else
              (`/Game/Blueprints/GI_GameInstanceMain.Lose Game` _as_gi_game_instance_main :!label _label_2))))
        (:`CastFailed`
          (goto _label_2))))))

(fn `Add Spline Meshes`
  (locals (SplineMeshComponent :type "SplineMeshComponent Object Reference"))
  (bind _ism (`self.ISM`))
  (for _index (range (+ (- (`InstancedStaticMeshComponent.GetInstanceCount` (`self.ISM`)) 2) 1))
    (bind _returnvalue (`AddComponent|NODE_AddSplineMeshComponent-2` :`bManualAttachment` true :`RelativeTransform` (`KismetMathLibrary.MakeTransform` (0.0 0.0 0.0) (struct) (1.5 1.5 1.5))))
    (bind _output_get (set `local.SplineMeshComponent` _returnvalue))
    (bind _outinstancetransform (`InstancedStaticMeshComponent.GetInstanceTransform` _ism (+ _index 1) true))
    (`SplineMeshComponent.SetStartPosition` _output_get (.location _outinstancetransform) true)
    (`SplineMeshComponent.SetStartTangent` _output_get (`KismetMathLibrary.GetForwardVector` (.rotation _outinstancetransform)) true)
    (bind _outinstancetransform_2 (`InstancedStaticMeshComponent.GetInstanceTransform` _ism _index true))
    (`SplineMeshComponent.SetEndPosition` _output_get (.location _outinstancetransform_2) true)
    (`SplineMeshComponent.SetEndTangent` _output_get (`KismetMathLibrary.GetForwardVector` (.rotation _outinstancetransform_2)) true)
    (`KismetArrayLibrary.Array_Add` (`self.SplineMeshComponents`) _output_get)))

(fn `SetSplineScale`
  (locals (SplineMeshComponent :type "SplineMeshComponent Object Reference"))
  (bind _splinemeshcomponents (`self.SplineMeshComponents`))
  (bind _splinemeshcomponent (`local.SplineMeshComponent`))
  (for _index (range (+ (- (`KismetArrayLibrary.Array_Length` _splinemeshcomponents) 2) 1))
    (set `local.SplineMeshComponent` (`|GetArrayItem` _splinemeshcomponents _index))
    (`SplineMeshComponent.SetStartScale` _splinemeshcomponent (`self.GetScale` _index) true)
    (`SplineMeshComponent.SetEndScale` _splinemeshcomponent (`self.GetScale` (+ _index 1)) true)))

(fn `UpdateSpline`
  (bind _ism (`self.ISM`))
  (for (_array_element _array_index) (`self.SplineMeshComponents`)
    (bind _outinstancetransform (`InstancedStaticMeshComponent.GetInstanceTransform` _ism (+ _array_index 1) true))
    (`SplineMeshComponent.SetStartPosition` _array_element (.location _outinstancetransform) true)
    (`SplineMeshComponent.SetStartTangent` _array_element (`KismetMathLibrary.GetForwardVector` (.rotation _outinstancetransform)) true)
    (bind _outinstancetransform_2 (`InstancedStaticMeshComponent.GetInstanceTransform` _ism _array_index true))
    (`SplineMeshComponent.SetEndPosition` _array_element (.location _outinstancetransform_2) true)
    (`SplineMeshComponent.SetEndTangent` _array_element (`KismetMathLibrary.GetForwardVector` (.rotation _outinstancetransform_2)) true)))

(fn `UserConstructionScript`
  (bind _ism (`self.ISM`))
  (`SceneComponent.K2_DetachFromComponent` _ism "KeepWorld" "KeepWorld" "KeepWorld" true)
  (`InstancedStaticMeshComponent.ClearInstances` _ism)
  (for _index (range (+ (`self.BalloonLength`) 1))
    (`InstancedStaticMeshComponent.AddInstance` (`self.ISM`) (`KismetMathLibrary.MakeTransform` (`KismetMathLibrary.MakeVector` (`KismetMathLibrary.Conv_IntToDouble` (* _index -75))) (struct) (`self.Instance Transform Scale`)) false))
  (`self.Add Spline Meshes`)
  (`self.SetSplineScale`))