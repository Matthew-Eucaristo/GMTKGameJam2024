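; BP_BalloonCutscene is a balloon actor for a cutscene that inflates in stages.
; The MakeBalloonBigger event takes a selection index and plays one of four timelines.
; Each timeline lerps the actor's uniform scale over a successive range, growing it from half size to just over double across the stages.
; BeginPlay, overlap, Tick and the construction script are empty.
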(event `Make Balloon Bigger`
  (params (Selection :type Integer))
  (switch `int` Selection
    (:`0`
      (bind (_direction _newtrack_0) (`Timeline|Scale` :!via `PlayFromStart`)
        (:`Update`
          (`self.SetActorScale3D` (`KismetMathLibrary.Conv_DoubleToVector` (`KismetMathLibrary.Lerp` 0.5 1.0 _newtrack_0))))))
    (:`1`
      (bind (_direction_2 _newtrack_0_2) (`Timeline|Timeline` :!via `PlayFromStart`)
        (:`Update`
          (`self.SetActorScale3D` (`KismetMathLibrary.Conv_DoubleToVector` (`KismetMathLibrary.Lerp` 1.0 1.5 _newtrack_0_2))))))
    (:`2`
      (bind (_direction_3 _newtrack_0_3) (`Timeline|Timeline_0` :!via `PlayFromStart`)
        (:`Update`
          (`self.SetActorScale3D` (`KismetMathLibrary.Conv_DoubleToVector` (`KismetMathLibrary.Lerp` 1.5 2.0 _newtrack_0_3))))))
    (:`3`
      (bind (_direction_4 _newtrack_0_4) (`Timeline|Timeline_1` :!via `PlayFromStart`)
        (:`Update`
          (`self.SetActorScale3D` (`KismetMathLibrary.Conv_DoubleToVector` (`KismetMathLibrary.Lerp` 2.0 2.2 _newtrack_0_4))))))))

(fn `UserConstructionScript`)