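; Main game mode that tracks a balloon gas energy meter and creates the energy bar and main menu widgets.
; Consuming gas succeeds only if enough remains, while generating gas clamps it to 0–1 and calls LoseGame on the game instance, cached at BeginPlay, when full.
; A FlipFlop alternately adds and removes the energy bar, whereas the main menu function only adds its widget, switching to UI-only input with a visible cursor.
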(event `self.ReceiveBeginPlay`
  (`|ExecutionSequence`
    (:`then_0`
      (bind _asgi_game_instance_main (cast `/Game/Blueprints/GI_GameInstanceMain` (`GameplayStatics.GetGameInstance`)))
      (set `self.As GI Game Instance Main` _asgi_game_instance_main))))

(fn `Add / Remove Balloon Energy Bar Widget`
  (returns (`WB Ref` :type "/Game/UI/WB_BalloonEnergyBar Object Reference"))
  (`/Engine/EditorBlueprintResources/StandardMacros.FlipFlop`
    (:`A`
      (bind _returnvalue (`|CreateWidget` "/Game/UI/WB_BalloonEnergyBar.WB_BalloonEnergyBar_C"))
      (bind _output_get (set `self.WB Balloon Energy Bar` _returnvalue))
      (`UserWidget.AddToViewport` _returnvalue 0)
      (`UserWidget.AddToViewport` _output_get 0)
      (return _output_get))
    (:`B`
      (`Widget.RemoveFromParent` (`self.WB Balloon Energy Bar`))
      (return null))))

(fn `Add / Remove Main Menu Widget`
  (returns (`WB Ref` :type "/Game/UI/WB_MainMenu Object Reference"))
  (bind _returnvalue (`GameplayStatics.GetPlayerController` 0))
  (bind _returnvalue_2 (`|CreateWidget` "/Game/UI/WB_MainMenu.WB_MainMenu_C"))
  (`UserWidget.AddToViewport` _returnvalue_2 0)
  (`WidgetBlueprintLibrary.SetInputMode_UIOnlyEx` _returnvalue _returnvalue_2)
  (set `PlayerController.bShowMouseCursor` true _returnvalue)
  (return _returnvalue_2))

(fn `Consume Gas`
  (params (`Gas Needed` :type "Float (double-precision)"))
  (returns (Succeed :type Boolean))
  (bind _returnvalue (- (`self.Gas Energy`) `Gas Needed`))
  (if (>= _returnvalue 0.0)
    (set `self.Gas Energy` _returnvalue)
    (return true)
    (else
      (return false))))

(fn `Generate Gas`
  (params (`Additional Gas Energy` :type "Float (double-precision)"))
  (bind _output_get (set `self.Gas Energy` (`KismetMathLibrary.FClamp` (+ `Additional Gas Energy` (`self.Gas Energy`)))))
  (if (== _output_get 1.0)
    (`KismetSystemLibrary.PrintString` "EXPLORDEEE" true true (struct :`R` 1.0 :`G` 0.008761 :`A` 1.0))
    (`/Game/Blueprints/GI_GameInstanceMain.Lose Game` (`self.As GI Game Instance Main`))))

(fn `UserConstructionScript`)