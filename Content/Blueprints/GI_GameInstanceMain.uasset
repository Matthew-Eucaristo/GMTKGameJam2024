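; Main Game Instance that runs background music across levels and shows the win and lose screens.
; On Init it caches the main player controller and uses short timers to spawn a persistent 2D music component and bind the StartNewLevel event.
; When a new level starts, it swaps the music track.
; WinGame and LoseGame each open their widget with cursor and UI-only input, guarded against repeat calls by a DoOnce that resets after a delay.
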(event `CustomEvent`
  (add `self.Start New Level` (delegate `Start New Level_Event`)))

(event `Start New Level_Event` :!signature `self.Start New Level`
  (params (Level :type Integer))
  (`AudioComponent.SetSound` (`self.MainSoundComponent`) "/Game/SFX/Music/Farting_Around_Cue.Farting_Around_Cue"))

(event `self.ReceiveInit`
  (`KismetSystemLibrary.K2_SetTimerDelegate` (delegate `SpawnSound2D`) 0.2)
  (`KismetSystemLibrary.K2_SetTimerDelegate` (delegate `CustomEvent`) 0.2)
  (bind _aspc_player_controller_main (cast `/Game/Blueprints/PC_PlayerControllerMain` (`GameplayStatics.GetPlayerController` 0)))
  (set `self.As PC Player Controller Main` _aspc_player_controller_main))

(event `SpawnSound2D`
  (bind _returnvalue (`GameplayStatics.SpawnSound2D` "/Game/SFX/Music/Goblin_Tinker_Soldier_Spy_Cue.Goblin_Tinker_Soldier_Spy_Cue" 1.0 1.0 0.0 null true))
  (set `self.MainSoundComponent` _returnvalue))

(event `Win Game`
  (bind _returnvalue (`GameplayStatics.GetPlayerController` 0))
  (`/Engine/EditorBlueprintResources/StandardMacros.DoOnce` false :!label _label
    (:`Completed`
      (`|ExecutionSequence`
        (:`then_0`
          (bind _returnvalue_2 (`|CreateWidget` "/Game/UI/WB_Win.WB_Win_C"))
          (`UserWidget.AddToViewport` _returnvalue_2 0)
          (set `PlayerController.bShowMouseCursor` true _returnvalue)
          (`WidgetBlueprintLibrary.SetInputMode_UIOnlyEx` _returnvalue _returnvalue_2))
        (:`then_1`
          (`KismetSystemLibrary.Delay` 2.0)
          (goto _label :!via `Reset`))))))

(event `Lose Game`
  (bind _returnvalue (`GameplayStatics.GetPlayerController` 0))
  (`/Engine/EditorBlueprintResources/StandardMacros.DoOnce` false :!label _label_2
    (:`Completed`
      (`|ExecutionSequence`
        (:`then_0`
          (bind _returnvalue_2 (`|CreateWidget` "/Game/UI/WB_Lose.WB_Lose_C"))
          (`UserWidget.AddToViewport` _returnvalue_2 0)
          (set `PlayerController.bShowMouseCursor` true _returnvalue)
          (`WidgetBlueprintLibrary.SetInputMode_UIOnlyEx` _returnvalue _returnvalue_2))
        (:`then_1`
          (`KismetSystemLibrary.Delay` 2.0)
          (goto _label_2 :!via `Reset`))))))