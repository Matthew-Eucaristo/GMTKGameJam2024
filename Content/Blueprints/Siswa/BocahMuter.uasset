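; BocahMuter is an ambient student character actor whose skeletal mesh travels along a spline.
; The construction script randomly picks one of four character meshes for visual variety.
; Each tick advances the distance by SplineSpeed and sets the mesh's local transform from the spline, with a yaw offset to correct facing.
; When Loop is enabled, the distance resets to zero past the spline's end.
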(event `self.ReceiveBeginPlay`)

(event `self.ReceiveTick`
  (params (DeltaSeconds :type "Float (single-precision)"))
  (bind _skeletalmesh (`self.SkeletalMesh`))
  (bind _returnvalue (`SplineComponent.GetTransformAtDistanceAlongSpline` (`self.Spline`) (`self.Distance along spline`) "Local" false))
  (set `self.Distance along spline` (+ (* DeltaSeconds (`self.spline speed`)) (`self.Distance along spline`)))
  (`SceneComponent.K2_SetRelativeTransform` _skeletalmesh (`KismetMathLibrary.MakeTransform` (.location _returnvalue) (`KismetMathLibrary.MakeRotator` (.roll (.rotation _returnvalue)) (.pitch (.rotation _returnvalue)) (+ (.yaw (.rotation _returnvalue)) -90.0)) (`SceneComponent.RelativeScale3D` _skeletalmesh)) false false)
  (if (`self.loop`)
    (if (> (`self.Distance along spline`) (`SplineComponent.GetSplineLength` (`self.Spline`)))
      (set `self.Distance along spline` 0.0))))

(fn `UserConstructionScript`
  (bind _skeletalmesh (`self.SkeletalMesh`))
  (`|ExecutionSequence`
    (:`then_0`
      (switch `int` (`KismetMathLibrary.RandomIntegerInRange` 0 3)
        (:`0`
          (`SkeletalMeshComponent.SetSkeletalMeshAsset` _skeletalmesh "/Game/Asset/Bocahan/Ch03_nonPBR.Ch03_nonPBR"))
        (:`1`
          (`SkeletalMeshComponent.SetSkeletalMeshAsset` _skeletalmesh "/Game/Asset/Bocahan/Ch09_nonPBR.Ch09_nonPBR"))
        (:`2`
          (`SkeletalMeshComponent.SetSkeletalMeshAsset` _skeletalmesh "/Game/Asset/Bocahan/Ch46_nonPBR.Ch46_nonPBR"))
        (:`3`
          (`SkeletalMeshComponent.SetSkeletalMeshAsset` _skeletalmesh "/Game/Asset/Bocahan/Ty.Ty"))))))